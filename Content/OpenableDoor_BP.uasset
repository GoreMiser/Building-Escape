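; An openable door actor that swings open and shut in response to OpenDoor's OnOpen and OnClose events.
; BeginPlay stores the starting rotation, and the DoorSwing timeline plays forward to open and reverses to close.
; Its OpenAngle track is applied as yaw combined with that initial rotation, so the swing is relative to the placed orientation.
; A Sound Timing event track plays the Doorlock sound at the actor's location.
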(event `self.ReceiveBeginPlay`
  ;[1 1 1] Set initial rotation
  (set `self.initRotation` (`self.K2_GetActorRotation`)))

(event `self.OpenDoor.onOpen`
  ;[1 1 1] Open or close the door
  (bind (_direction _openangle) (`Timeline|Door Swing` :!label _label)
    (:`Update`
      (`self.K2_SetActorRotation` (`KismetMathLibrary.ComposeRotators` (`KismetMathLibrary.MakeRotator` 0.0 0.0 _openangle) (`self.initRotation`))))
    (:`Sound Timing`
      (`GameplayStatics.PlaySoundAtLocation` "/Game/Audio/door-lock.door-lock" (`self.K2_GetActorLocation`)))))

(event `self.OpenDoor.onClose`
  ;[1 1 1] Open or close the door
  (goto _label :!via `Reverse`))

(fn `UserConstructionScript`)